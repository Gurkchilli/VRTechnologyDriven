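; Cylinder2_Blueprint is an overlap trigger that toggles the visibility of SpookyMan, Text and Box in the game.
; On every ActorBeginOverlap, with no filter on the overlapping actor, it reads SpookyMan's Hidden flag and shows or hides all three together.
; SpookyMan's state alone drives the toggle, so Text and Box are set to match it regardless of their own visibility.
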(event `self.ReceiveActorBeginOverlap`
  (params (OtherActor :type "Actor Object Reference"))
  (if (`Actor.bHidden` (`self.SpookyMan`))
    (`|ExecutionSequence`
      (:`then_0`
        (`self.SetActorHiddenInGame` (`self.SpookyMan`) false))
      (:`then_1`
        (`self.SetActorHiddenInGame` (`self.Text`) false))
      (:`then_2`
        (`self.SetActorHiddenInGame` (`self.Box`) false)))
    (else
      (`|ExecutionSequence`
        (:`then_0`
          (`self.SetActorHiddenInGame` (`self.SpookyMan`) true))
        (:`then_1`
          (`self.SetActorHiddenInGame` (`self.Text`) true))
        (:`then_2`
          (`self.SetActorHiddenInGame` (`self.Box`) true))))))

(fn `UserConstructionScript`)