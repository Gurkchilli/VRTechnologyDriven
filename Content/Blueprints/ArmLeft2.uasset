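; ArmLeft2 is an actor Blueprint for an arm that the player poses with the keyboard, rotating its shoulder, elbow and hand.
; BeginPlay enables input, and number keys 1 to 8 each open a gate while held and close it on release.
; Tick feeds every gate through sequences, so open gates add a fixed local rotation to their joint each frame, independent of delta time.
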(event `Key|One`
  (params (Key :type "Key Structure"))
  ;[1 1 1] Shoulder
  (:`Pressed`
    (goto _label :!via `Open`))
  (:`Released`
    (goto _label :!via `Close`)))

(event `Key|Two`
  (params (Key :type "Key Structure"))
  ;[1 1 1] Shoulder
  (:`Pressed`
    (goto _label_2 :!via `Open`))
  (:`Released`
    (goto _label_2 :!via `Close`)))

(event `Key|Seven`
  (params (Key :type "Key Structure"))
  ;[1 1 1] Shoulder
  (:`Pressed`
    (goto _label_3 :!via `Open`))
  (:`Released`
    (goto _label_3 :!via `Close`)))

(event `self.ReceiveBeginPlay`
  (`self.EnableInput` (`GameplayStatics.GetPlayerController` 0)))

(event `self.ReceiveTick`
  (params (DeltaSeconds :type "Float (single-precision)"))
  (`|ExecutionSequence`
    (:`then_0`
      ;[1 1 1] Shoulder
      (`|ExecutionSequence`
        (:`then_0`
          (`/Engine/EditorBlueprintResources/StandardMacros.Gate` true :!label _label
            (:`Exit`
              (`SceneComponent.K2_AddLocalRotation` (`self.ShoulderPivot`) (struct :`Roll` 1.0) false false))))
        (:`then_1`
          (`/Engine/EditorBlueprintResources/StandardMacros.Gate` true :!label _label_2
            (:`Exit`
              (`SceneComponent.K2_AddLocalRotation` (`self.ShoulderPivot`) (struct :`Roll` -1.0) false false))))
        (:`then_2`
          (`/Engine/EditorBlueprintResources/StandardMacros.Gate` true :!label _label_3
            (:`Exit`
              (`SceneComponent.K2_AddLocalRotation` (`self.ShoulderPivot`) (struct :`Yaw` 1.0) false false))))
        (:`then_3`
          (`/Engine/EditorBlueprintResources/StandardMacros.Gate` true :!label _label_4
            (:`Exit`
              (`SceneComponent.K2_AddLocalRotation` (`self.ShoulderPivot`) (struct :`Yaw` -1.0) false false))))))
    (:`then_1`
      ;[1 1 1] Elbow
      (`|ExecutionSequence`
        (:`then_0`
          (`/Engine/EditorBlueprintResources/StandardMacros.Gate` true :!label _label_5
            (:`Exit`
              (`SceneComponent.K2_AddLocalRotation` (`self.ElbowPivot`) (struct :`Roll` 1.0) false false))))
        (:`then_1`
          (`/Engine/EditorBlueprintResources/StandardMacros.Gate` true :!label _label_6
            (:`Exit`
              (`SceneComponent.K2_AddLocalRotation` (`self.ElbowPivot`) (struct :`Roll` -1.0) false false))))))
    (:`then_2`
      ;[1 1 1] Hand
      (`|ExecutionSequence`
        (:`then_0`
          (`/Engine/EditorBlueprintResources/StandardMacros.Gate` true :!label _label_7
            (:`Exit`
              (`SceneComponent.K2_AddLocalRotation` (`self.Hnad`) (struct :`Pitch` 1.0) false false))))
        (:`then_1`
          (`/Engine/EditorBlueprintResources/StandardMacros.Gate` true :!label _label_8
            (:`Exit`
              (`SceneComponent.K2_AddLocalRotation` (`self.Hnad`) (struct :`Pitch` -1.0) false false))))))))

(event `Key|Eight`
  (params (Key :type "Key Structure"))
  ;[1 1 1] Shoulder
  (:`Pressed`
    (goto _label_4 :!via `Open`))
  (:`Released`
    (goto _label_4 :!via `Close`)))

(event `Key|Three`
  (params (Key :type "Key Structure"))
  ;[1 1 1] Elbow
  (:`Pressed`
    (goto _label_5 :!via `Open`))
  (:`Released`
    (goto _label_5 :!via `Close`)))

(event `Key|Four`
  (params (Key :type "Key Structure"))
  ;[1 1 1] Elbow
  (:`Pressed`
    (goto _label_6 :!via `Open`))
  (:`Released`
    (goto _label_6 :!via `Close`)))

(event `Key|Five`
  (params (Key :type "Key Structure"))
  ;[1 1 1] Hand
  (:`Pressed`
    (goto _label_7 :!via `Open`))
  (:`Released`
    (goto _label_7 :!via `Close`)))

(event `Key|Six`
  (params (Key :type "Key Structure"))
  ;[1 1 1] Hand
  (:`Pressed`
    (goto _label_8 :!via `Open`))
  (:`Released`
    (goto _label_8 :!via `Close`)))

(fn `UserConstructionScript`)