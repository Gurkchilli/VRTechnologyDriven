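; Trigger box that swaps an in-level text and reveals a button when a box reaches it.
; The first overlap by an actor tagged "Box" passes a DoOnce, hiding OldText and showing NewText, ButtonPole and Button.
; A disconnected chain that would spawn Box_Blueprint at every TargetPoint remains in the graph but never runs.
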(event `self.ReceiveActorBeginOverlap`
  (params (OtherActor :type "Actor Object Reference"))
  (if (`self.ActorHasTag` OtherActor "Box")
    (`/Engine/EditorBlueprintResources/StandardMacros.DoOnce` false
      (:`Completed`
        (`|ExecutionSequence`
          (:`then_0`
            (`self.SetActorHiddenInGame` (`self.OldText`) true))
          (:`then_1`
            (`self.SetActorHiddenInGame` (`self.NewText`) false))
          (:`then_2`
            (`self.SetActorHiddenInGame` (`self.ButtonPole`) false))
          (:`then_3`
            (`self.SetActorHiddenInGame` (`self.Button`) false)))))))

(fn `UserConstructionScript`)