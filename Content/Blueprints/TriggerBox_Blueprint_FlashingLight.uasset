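; Trigger box Blueprint that makes a spotlight flash once an actor overlaps it.
; Overlap plays a timeline unless IsPlaying is set, scaling its Brightness track into the light's intensity and restarting on finish to loop indefinitely.
; The timeline's Trigger Toggle event flips IsPlaying through a FlipFlop.
; A light color update from the timeline's LightColor track exists but is disconnected, so only intensity changes.
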(event `self.ReceiveActorBeginOverlap`
  (params (OtherActor :type "Actor Object Reference"))
  (if (not (`self.IsPlaying`))
    (bind (_direction _brightness _light_color) (`Timeline|Timeline_0` :!label _label)
      (:`Update`
        (`LightComponent.SetIntensity` (`Light.LightComponent` (`self.SpotLight`)) (* _brightness 20.0)))
      (:`Finished`
        (if true
          (goto _label :!via `PlayFromStart`)))
      (:`Trigger Toggle`
        (bind _isa (`/Engine/EditorBlueprintResources/StandardMacros.FlipFlop`)
          (:`A`
            _)
          (:`B`
            _))
        (set `self.IsPlaying` _isa)))))

(fn `UserConstructionScript`)