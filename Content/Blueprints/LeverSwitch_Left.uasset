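; Lever switch actor that rotates a linked object according to how far its handle is tilted.
; Each Tick it reads the handle's pitch relative to the actor and, beyond a small dead zone either way, adds a fixed local rotation step to the LinkedObject's root component.
; The tilt direction sets the rotation direction, and the step is not scaled by delta time, so speed depends on frame rate.
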(event `self.ReceiveTick`
  (params (DeltaSeconds :type "Float (single-precision)"))
  (bind _pitch (.pitch (`KismetMathLibrary.InverseTransformRotation` (`self.GetTransform`) (`SceneComponent.K2_GetComponentRotation` (`self.Handle`)))))
  (`|ExecutionSequence`
    (:`then_0`
      (if (> _pitch 10.0)
        (`SceneComponent.K2_AddLocalRotation` (`Actor.RootComponent` (`self.LinkedObject`)) (struct :`Yaw` -0.3) false false)))
    (:`then_1`
      (if (> -10.0 _pitch)
        (`SceneComponent.K2_AddLocalRotation` (`Actor.RootComponent` (`self.LinkedObject`)) (struct :`Yaw` 0.3) false false)))))

(fn `UserConstructionScript`
  (`parent.UserConstructionScript`))