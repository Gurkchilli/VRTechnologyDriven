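; Lever actor that keeps its position along the Y axis between a positive and a negative drag limit.
; Each Tick it reads its world location, prints it, and clamps Y by writing the result back as a relative location.
; It also derives a rounded output from Y divided by the positive limit, but only feeds it to a PrintString with screen and log output disabled.
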(event `self.ReceiveBeginPlay`)

(event `self.ReceiveTick`
  (params (DeltaSeconds :type "Float (single-precision)"))
  (bind _drag_length (`self.Drag_Length`))
  (bind _drag_length_negative (`self.Drag_length_negative`))
  (bind _returnvalue (`self.K2_GetActorLocation` self))
  (bind _x (.x _returnvalue))
  (bind _y (.y _returnvalue))
  (bind _z (.z _returnvalue))
  (`KismetSystemLibrary.PrintString` (`KismetStringLibrary.Conv_VectorToString` _returnvalue) true false)
  (if (> _y _drag_length)
    (`self.K2_SetActorRelativeLocation` (`KismetMathLibrary.MakeVector` _x _drag_length _z))
    (elif (> _drag_length_negative _y)
      (`self.K2_SetActorRelativeLocation` (`KismetMathLibrary.MakeVector` _x _drag_length_negative _z))))
  (`KismetSystemLibrary.PrintString` (`KismetStringLibrary.Conv_IntToString` (`KismetMathLibrary.Round` (/ _y _drag_length))) false false))

(fn `UserConstructionScript`)