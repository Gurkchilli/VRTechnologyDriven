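; Right arm actor that lets the player rotate its shoulder, elbow and hand joints from the keyboard.
; BeginPlay enables input from the first player controller, and key press and release events open and close one gate per rotation direction.
; Tick feeds every gate, so a held key adds a fixed local rotation each frame, independent of delta time.
; The shoulder turns on two axes, while elbow and hand turn on one each.
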(event `Key|Q`
  (params (Key :type "Key Structure"))
  ;[1 1 1] Shoulder
  (:`Pressed`
    (goto _label :!via `Open`))
  (:`Released`
    (goto _label :!via `Close`)))

(event `Key|E`
  (params (Key :type "Key Structure"))
  ;[1 1 1] Shoulder
  (:`Pressed`
    (goto _label_2 :!via `Open`))
  (:`Released`
    (goto _label_2 :!via `Close`)))

(event `Key|Z`
  (params (Key :type "Key Structure"))
  ;[1 1 1] Shoulder
  (:`Pressed`
    (goto _label_3 :!via `Open`))
  (:`Released`
    (goto _label_3 :!via `Close`)))

(event `self.ReceiveBeginPlay`
  (`self.EnableInput` (`GameplayStatics.GetPlayerController` 0)))

(event `Key|X`
  (params (Key :type "Key Structure"))
  ;[1 1 1] Shoulder
  (:`Pressed`
    (goto _label_4 :!via `Open`))
  (:`Released`
    (goto _label_4 :!via `Close`)))

(event `self.ReceiveTick`
  (params (DeltaSeconds :type "Float (single-precision)"))
  (`|ExecutionSequence`
    (:`then_0`
      ;[1 1 1] Shoulder
      (`|ExecutionSequence`
        (:`then_0`
          (`/Engine/EditorBlueprintResources/StandardMacros.Gate` true :!label _label
            (:`Exit`
              (`SceneComponent.K2_AddLocalRotation` (`self.Shoulder`) (struct :`Roll` 1.0) false false))))
        (:`then_1`
          (`/Engine/EditorBlueprintResources/StandardMacros.Gate` true :!label _label_2
            (:`Exit`
              (`SceneComponent.K2_AddLocalRotation` (`self.Shoulder`) (struct :`Roll` -1.0) false false))))
        (:`then_2`
          (`/Engine/EditorBlueprintResources/StandardMacros.Gate` true :!label _label_3
            (:`Exit`
              (`SceneComponent.K2_AddLocalRotation` (`self.Shoulder`) (struct :`Yaw` 1.0) false false))))
        (:`then_3`
          (`/Engine/EditorBlueprintResources/StandardMacros.Gate` true :!label _label_4
            (:`Exit`
              (`SceneComponent.K2_AddLocalRotation` (`self.Shoulder`) (struct :`Yaw` -1.0) false false))))))
    (:`then_1`
      ;[1 1 1] Elbow
      (`|ExecutionSequence`
        (:`then_0`
          (`/Engine/EditorBlueprintResources/StandardMacros.Gate` true :!label _label_5
            (:`Exit`
              (`SceneComponent.K2_AddLocalRotation` (`self.Elbow1`) (struct :`Roll` 1.0) false false))))
        (:`then_1`
          (`/Engine/EditorBlueprintResources/StandardMacros.Gate` true :!label _label_6
            (:`Exit`
              (`SceneComponent.K2_AddLocalRotation` (`self.Elbow1`) (struct :`Roll` -1.0) false false))))))
    (:`then_2`
      ;[1 1 1] Hand
      (`|ExecutionSequence`
        (:`then_0`
          (`/Engine/EditorBlueprintResources/StandardMacros.Gate` true :!label _label_7
            (:`Exit`
              (`SceneComponent.K2_AddLocalRotation` (`self.Hnad`) (struct :`Pitch` 1.0) false false))))
        (:`then_1`
          (`/Engine/EditorBlueprintResources/StandardMacros.Gate` true :!label _label_8
            (:`Exit`
              (`SceneComponent.K2_AddLocalRotation` (`self.Hnad`) (struct :`Pitch` -1.0) false false))))))))

(event `Key|Divide`
  (params (Key :type "Key Structure"))
  ;[1 1 1] Elbow
  (:`Pressed`
    (goto _label_5 :!via `Open`))
  (:`Released`
    (goto _label_5 :!via `Close`)))

(event `Key|Multiply`
  (params (Key :type "Key Structure"))
  ;[1 1 1] Elbow
  (:`Pressed`
    (goto _label_6 :!via `Open`))
  (:`Released`
    (goto _label_6 :!via `Close`)))

(event `Key|Subtract`
  (params (Key :type "Key Structure"))
  ;[1 1 1] Hand
  (:`Pressed`
    (goto _label_7 :!via `Open`))
  (:`Released`
    (goto _label_7 :!via `Close`)))

(event `Key|Add`
  (params (Key :type "Key Structure"))
  ;[1 1 1] Hand
  (:`Pressed`
    (goto _label_8 :!via `Open`))
  (:`Released`
    (goto _label_8 :!via `Close`)))

(fn `UserConstructionScript`)