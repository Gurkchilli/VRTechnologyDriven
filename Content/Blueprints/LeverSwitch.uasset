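; LeverSwitch is a lever actor that slides a linked object back and forth according to the tilt of its Handle.
; Each Tick converts the Handle's world rotation into actor-local space and compares its pitch against a small symmetric dead zone.
; Beyond either threshold, LinkedObject's root moves a fixed local step left or right per frame, independent of delta time, with sweep only on the left move.
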(event `self.ReceiveTick`
  (params (DeltaSeconds :type "Float (single-precision)"))
  (bind _pitch (.pitch (`KismetMathLibrary.InverseTransformRotation` (`self.GetTransform`) (`SceneComponent.K2_GetComponentRotation` (`self.Handle`)))))
  (`|ExecutionSequence`
    (:`then_0`
      (if (> _pitch 2.0)
        (`SceneComponent.K2_AddLocalTransform` (`Actor.RootComponent` (`self.LinkedObject`)) (`KismetMathLibrary.Conv_VectorToTransform` (* (`KismetMathLibrary.Vector_Left`) 3)) true false) ; Walk Forward
      ))
    (:`then_1`
      (if (> -2.0 _pitch)
        (`SceneComponent.K2_AddLocalTransform` (`Actor.RootComponent` (`self.LinkedObject`)) (`KismetMathLibrary.Conv_VectorToTransform` (* (`KismetMathLibrary.Vector_Right`) 3)) false false) ; Walk Backwards
      ))))

(fn `UserConstructionScript`)