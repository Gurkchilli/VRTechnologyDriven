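; Flashing light actor that varies the intensity of its Light through a timeline.
; On BeginPlay, if IsPlaying is false, it plays Timeline_0, whose Brightness track is scaled and sent to the light's intensity each update.
; The timeline's Toggle event drives a FlipFlop that writes IsPlaying, which nothing rechecks after startup.
; A node for setting light color from the timeline exists but is never run.
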(event `self.ReceiveBeginPlay`
  (if (not (`self.IsPlaying`))
    (bind (_direction _brightness _light_color) (`Timeline|Timeline_0`)
      (:`Update`
        (`LightComponent.SetIntensity` (`self.Light`) (* _brightness 20.0)))
      (:`Trigger Toggle`
        (bind _isa (`/Engine/EditorBlueprintResources/StandardMacros.FlipFlop`)
          (:`A`
            _)
          (:`B`
            _))
        (set `self.IsPlaying` _isa)))))

(event `self.ReceiveTick`
  (params (DeltaSeconds :type "Float (single-precision)")))

(fn `UserConstructionScript`)